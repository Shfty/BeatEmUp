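; Player controller for a beat 'em up that handles quitting on Escape, input device tracking, rumble and level streaming.
; Any key press or release updates whether the keyboard is in use, which gates playback through the force feedback component.
; On BeginPlay it flags the BeCK player state as the server player when this controller is local and on the server.
; LoadLevel marks a named streaming level to be loaded and visible.
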(event EventBeginPlay
  (bind _asbp_be_ckplayer_state (Utilities|Casting|CastToBP_BeCKPlayerState (Variables|GetPlayerState)))
  (Variables|/BeCK/Blueprints/GameplayFramework/BP_BeCKPlayerState.BP_BeCKPlayerState_C|SetIsServerPlayer _asbp_be_ckplayer_state (and (Pawn|IsLocalPlayerController) (Networking|IsServer))))

(event Input|KeyboardEvents|Escape
  (params (Key :type Key%20Structure :default "AnyKey"))
  ;[1 1 1] Quit handler
  (:Pressed
    (Game|QuitGame 0 "Quit")))

(event Input|KeyboardEvents|AnyKey
  (params (Key :type Key%20Structure :default "AnyKey"))
  ;[1 1 1] Determine current device on input
  (:Pressed
    (Variables|Default|SetIsUsingKeyboard (Class|KismetInputLibrary|KeyIsKeyboardKey Key) :!label _label))
  (:Released
    (goto _label)))

(fn ConstructionScript)

(fn PlayForceFeedbackEffect
  (params (InputPin :type Force%20Feedback%20Effect%20Object%20Reference))
  (bind _forcefeedback (Variables|Default|GetForceFeedback))
  (if (not (Variables|Default|GetIsUsingKeyboard))
    (Class|ForceFeedbackComponent|SetForceFeedbackEffect _forcefeedback InputPin)
    (Audio|Components|Audio|Play _forcefeedback 0.0)))