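; Scratch test actor that blends the view between perspective and orthographic projection and checks that mouse picking still works during the blend.
; BeginPlay builds both matrices from the viewport size; Tick oscillates a sine alpha through a float curve to interpolate and apply a custom projection matrix.
; The same matrix drives a custom screen-to-world deprojection for a cursor line trace, placing the static mesh at the hit aligned to the ray, or hiding it.
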(event EventBeginPlay
  (bind _returnvalue (Viewport|GetViewportSize))
  (bind _returnvalue_2 (Viewport|GetViewportSize))
  (Utilities|Struct|SetmembersinMatrixData (Variables|Default|GetPerspectiveMatrix) (Class|OrthoHMDFunctionLibrary|MakePerspectiveMatrix 45.0 (.x _returnvalue_2) (.y _returnvalue_2) 0.01 true))
  (Utilities|Struct|SetmembersinMatrixData (Variables|Default|GetOrthoMatrix) (Class|OrthoHMDFunctionLibrary|MakeOrthoMatrix (.x _returnvalue) (.y _returnvalue) 0.01 1e+04 true)))

(event EventTick
  (params (DeltaSeconds :type Float%20%28single-precision%29))
  (bind _returnvalue (Game|GetPlayerController 0))
  (bind _projectionmatrix (Variables|Default|GetProjectionMatrix))
  (bind _staticmesh (Variables|Default|GetStaticMesh))
  (bind _matrix (Utilities|Struct|BreakMatrixData _projectionmatrix))
  (bind (_locationx _locationy) (Game|Player|GetMousePosition _returnvalue))
  (bind (_worldposition _worlddirection _returnvalue_2) (Class|OrthoHMDFunctionLibrary|CustomDeprojectScreentoWorld _returnvalue (Math|Vector2D|MakeVector2D _locationx _locationy) _matrix))
  (Utilities|FlowControl|Sequence
    (:then_0
      (Variables|Default|SetLerpAlpha (* (+ (Math|Trig|Sin(Radians) (Utilities|Time|GetTimeSeconds)) 1.0) 0.5)))
    (:then_1
      (Class|OrthoHMDFunctionLibrary|SetCustomProjectionMatrix (Class|OrthoHMDFunctionLibrary|InterpolateMatrices (Utilities|Struct|BreakMatrixData (Variables|Default|GetPerspectiveMatrix)) (Utilities|Struct|BreakMatrixData (Variables|Default|GetOrthoMatrix)) (Math|Float|Clamp(Float) (Math|Curves|GetFloatValue (Variables|Default|GetProjectionInterpolationCurve) (Variables|Default|GetLerpAlpha)))))
      (Utilities|Struct|SetmembersinMatrixData (Variables|Default|GetProjectionMatrix) (Class|OrthoHMDFunctionLibrary|InterpolateMatrices (Utilities|Struct|BreakMatrixData (Variables|Default|GetPerspectiveMatrix)) (Utilities|Struct|BreakMatrixData (Variables|Default|GetOrthoMatrix)) (Math|Float|Clamp(Float) (Math|Curves|GetFloatValue (Variables|Default|GetProjectionInterpolationCurve) (Variables|Default|GetLerpAlpha))))))
    (:then_2
      (if _returnvalue_2
        (bind (_outhit _returnvalue_3) (Collision|LineTraceByChannel _worldposition (+ _worldposition (* _worlddirection 1e+05)) "TraceTypeQuery1" false 0 "None"))
        (if _returnvalue_3
          (Rendering|SetVisibility _staticmesh true false)
          (Transformation|SetWorldLocationAndRotation _staticmesh (.ImpactPoint (Collision|BreakHitResult _outhit)) (Math|Rotator|MakeRotfromX _worlddirection) false false)
          (else
            (Rendering|SetVisibility _staticmesh false false :!label _label)))
        (else
          (goto _label))))))

(fn ConstructionScript)