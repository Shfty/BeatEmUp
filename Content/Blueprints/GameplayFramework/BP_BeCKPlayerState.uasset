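; BP_BeCKPlayerState is a player state that holds health and a measured framerate, and relays input presses.
; Construction sets Health to MaxHealth, and HandleInputPressed forwards its input through InputPressed.
; Tick counts frames and elapsed time to compute an average framerate once just over half a second accumulates.
; Only the non-authority branch passes that value to SetFramerateCounter and resets the counters.
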(event Custom|HandleInputPressed
  (params (Input :type BeatEmUpInputSchema%20Enum))
  (Default|CallInputPressed Input))

(event Custom|SetFramerateCounter
  (params (NewParam :type Float%20%28single-precision%29))
  (Variables|FramerateCounter|Replicated|SetFramerate NewParam))

(event EventTick
  (params (DeltaSeconds :type Float%20%28single-precision%29))
  (CallFunction|UpdateFramerateCounter DeltaSeconds))

(fn ConstructionScript
  (Variables|Health|Replicated|SetHealth (Variables|Health|GetMaxHealth)))

(fn UpdateFramerateCounter
  (params (DeltaTime :type Float%20%28single-precision%29))
  (bind _result (Math|Integer|IncrementInt (Variables|FramerateCounter|GetTickCounter))
    (:%20%20
      (bind _output_get (Variables|FramerateCounter|SetTimeCounter (+ (Variables|FramerateCounter|GetTimeCounter) DeltaTime)))
      (if (> _output_get 0.5)
        (bind _output_get_2 (Variables|FramerateCounter|Replicated|SetFramerate (/ (Math|Conversions|ToFloat(Integer) _result) (Variables|FramerateCounter|GetTimeCounter))))
        (Networking|SwitchHasAuthority
          (:Remote
            (CallFunction|SetFramerateCounter _output_get_2)
            (Variables|FramerateCounter|SetTickCounter 0)
            (Variables|FramerateCounter|SetTimeCounter 0.0)))))))