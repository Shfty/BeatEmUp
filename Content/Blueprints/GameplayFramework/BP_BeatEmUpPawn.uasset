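; Player pawn for a beat 'em up, adding camera-relative movement, hit rumble and room-based network relevancy.
; Move input feeds BeatEmUpMovement along camera axes, with vertical input skewed sideways by the camera manager's ShearFactor.
; Hit effects extend the parent's with controller force feedback.
; It is relevant to viewers whose current or connected rooms contain it, deferring to parent logic when no room is found.
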(event EventAddMovementVectors
  (bind _moveinput (Variables|Default|GetMoveInput))
  (bind _y (Math|Vector2D|BreakVector2D _moveinput))
  (bind _asplayer_controller (Utilities|Casting|CastToPlayerController (Pawn|GetController)))
  (Utilities|FlowControl|Sequence
    (:then_0
      (Class|PawnMovementComponent|AddInputVector (Variables|Default|GetBeatEmUpMovement) (* (Math|Vector|GetRightVector (Camera|GetCameraRotation (Variables|/Script/Engine.PlayerController|GetPlayerCameraManager _asplayer_controller))) (.X (Math|Vector2D|BreakVector2D (Variables|Default|GetMoveInput)))) false))
    (:then_1
      (Class|PawnMovementComponent|AddInputVector (Variables|Default|GetBeatEmUpMovement) (+ (* (Math|Vector|GetForwardVector (Camera|GetCameraRotation (Variables|/Script/Engine.PlayerController|GetPlayerCameraManager _asplayer_controller))) _y) (* (Math|Vector|GetRightVector (Camera|GetCameraRotation (Variables|/Script/Engine.PlayerController|GetPlayerCameraManager _asplayer_controller))) (* _y (* (.X (Math|Vector2D|BreakVector2D (Variables|/Game/Blueprints/GameplayFramework/BP_BeatEmUpCameraManager.BP_BeatEmUpCameraManager_C|GetShearFactor (.AsBP%20Beat%20Em%20Up%20Camera%20Manager (Utilities|Casting|CastToBP_BeatEmUpCameraManager (Game|GetPlayerCameraManager 0)))))) -1.0)))) false))))

(event EventSpawnHitEffects
  (params (ParticleSystem :type Particle%20System%20Object%20Reference) (SoundEffect :type Sound%20Base%20Object%20Reference) (Location :type Vector) (Impulse :type Vector))
  (|CallParentFunction ParticleSystem SoundEffect Location Impulse)
  (bind _asbp_beat_em_up_player_controller (Utilities|Casting|CastToBP_BeatEmUpPlayerController (Pawn|GetController)))
  (Default|PlayForceFeedbackEffect _asbp_beat_em_up_player_controller "/Game/ForceFeedback/HitForceFeedback.HitForceFeedback"))

(fn ConstructionScript
  (|CallParentFunction))

(fn IsNetworkRelevantfor
  (params (RealViewer :type Actor%20Object%20Reference) (ViewTarget :type Actor%20Object%20Reference) (SrcLocation :type Vector%20%28by%20ref%29))
  (bind _self self)
  (bind _aspawn (Utilities|Casting|CastToPawn ViewTarget)
    (:then
      (bind _asbp_beat_em_up_player_state (Utilities|Casting|CastToBP_BeatEmUpPlayerState (Variables|/Script/Engine.Pawn|GetPlayerState _aspawn))
        (:then
          (Utilities|IsValid (Variables|/Game/Blueprints/GameplayFramework/BP_BeatEmUpPlayerState.BP_BeatEmUpPlayerState_C|GetCurrentRoom _asbp_beat_em_up_player_state)
            (:Is%20Valid
              (return (or (Default|ContainsActor (Variables|/Game/Blueprints/GameplayFramework/BP_BeatEmUpPlayerState.BP_BeatEmUpPlayerState_C|GetCurrentRoom _asbp_beat_em_up_player_state) _self) (Default|ConnectedRoomsContainActor (Variables|/Game/Blueprints/GameplayFramework/BP_BeatEmUpPlayerState.BP_BeatEmUpPlayerState_C|GetCurrentRoom _asbp_beat_em_up_player_state) _self))))
            (:Is%20Not%20Valid
              _)))
        (:CastFailed
          _)))
    (:CastFailed
      _))
  (bind _returnvalue (|CallParentFunction RealViewer ViewTarget SrcLocation))
  (return _returnvalue))