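; Box volume marking a room that drives sublevel streaming and sky visibility in a multiplayer beat-em-up.
; On pawn overlap it sets the player state's CurrentRoom and the skybox fade target from ShowSky.
; The server loads its sublevel at BeginPlay; clients load the local pawn's room and ConnectedRooms, unloading neighbours' other connections that lack that pawn.
; The construction script draws long-lived debug arrows showing room connections.
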(event OnComponentBeginOverlap(Box)
  (params (OverlappedComponent :type Primitive%20Component%20Object%20Reference) (OtherActor :type Actor%20Object%20Reference) (OtherComp :type Primitive%20Component%20Object%20Reference) (OtherBodyIndex :type Integer) (bFromSweep :type Boolean) (SweepResult :type Hit%20Result%20Structure%20%28by%20ref%29))
  (CallFunction|HandleBeginOverlap OtherActor))

(event EventBeginPlay
  (bind _sublevelname (Variables|Default|GetSublevelName))
  (bind _returnvalue (Class|GameplayStatics|GetStreamingLevel _sublevelname))
  (Utilities|FlowControl|Sequence
    (:then_0
      (Utilities|IsValid _returnvalue
        (:Is%20Valid
          (Variables|/Script/Engine.LevelStreaming|SetbShouldBlockOnLoad _returnvalue false)
          (if (Networking|IsServer)
            (CallFunction|SetLevelState true)))))
    (:then_1
      (for _array_element (Collision|GetOverlappingActors (Variables|Default|GetBox) "/Script/Engine.Pawn" :!class /Script/Engine.PrimitiveComponent)
        (CallFunction|HandleBeginOverlap _array_element)))))

(fn ConstructionScript
  (bind _returnvalue (Transformation|GetActorLocation))
  (bind _returnvalue_2 (Math|Float|MakeLiteralFloat 3e+07))
  (bind _returnvalue_3 (+ _returnvalue "0, 0,100.000000"))
  (Utilities|FlowControl|Sequence
    (:then_0
      (Components|Box|SetBoxExtent (Variables|Default|GetBox) (Variables|Default|GetBoxExtent) true))
    (:then_1
      (bind _outactors (Actor|GetAllActorsOfClass "BP_RoomVolume_C"))
      (if (== (Utilities|Array|Get(acopy) _outactors) self)
        (Rendering|Debug|FlushPersistentDebugLines)))
    (:then_2
      (for _array_element (Variables|Default|GetConnectedRooms)
        (Rendering|Debug|DrawDebugLine _returnvalue_3 (Transformation|GetActorLocation _array_element) "(R=1.000000,G=1.000000,B=1.000000,A=1.000000)" _returnvalue_2 0.0)
        (Rendering|Debug|DrawDebugSphere _returnvalue_3 1e+01 12 "(R=1.000000,G=1.000000,B=1.000000,A=1.000000)" _returnvalue_2)
        (Rendering|Debug|DrawDebugBox (Transformation|GetActorLocation _array_element) "10.000000,10.000000,10.000000" "(R=1.000000,G=1.000000,B=1.000000,A=1.000000)" "0, 0, 0" _returnvalue_2 0.0)
        (Class|KismetSystemLibrary|DrawDebugConeinDegrees (+ _returnvalue_3 (* (Math|Vector|Normalize (- _returnvalue_3 (Transformation|GetActorLocation _array_element))) (* (Math|Vector|VectorLength (- _returnvalue_3 (Transformation|GetActorLocation _array_element))) -0.25))) (Math|Vector|Normalize (- _returnvalue_3 (Transformation|GetActorLocation _array_element))) 1e+02 3e+01 3e+01 12 "(R=1.000000,G=1.000000,B=1.000000,A=1.000000)" _returnvalue_2 0.0)
        (Class|KismetSystemLibrary|DrawDebugConeinDegrees (+ _returnvalue_3 (* (Math|Vector|Normalize (- _returnvalue_3 (Transformation|GetActorLocation _array_element))) (* (Math|Vector|VectorLength (- _returnvalue_3 (Transformation|GetActorLocation _array_element))) -0.75))) (Math|Vector|Normalize (- _returnvalue_3 (Transformation|GetActorLocation _array_element))) 1e+02 3e+01 3e+01 12 "(R=1.000000,G=1.000000,B=1.000000,A=1.000000)" _returnvalue_2 0.0)))))

(fn SetLevelState
  (params (Loaded :type Boolean))
  (bind _sublevelname (Variables|Default|GetSublevelName))
  (bind _returnvalue (Class|GameplayStatics|GetStreamingLevel _sublevelname))
  (Utilities|IsValid _returnvalue
    (:Is%20Valid
      (Variables|/Script/Engine.LevelStreaming|SetbShouldBeLoaded _returnvalue Loaded)
      (Variables|/Script/Engine.LevelStreaming|SetbShouldBeVisible _returnvalue Loaded))))

(fn HandleBeginOverlap
  (params (Object :type Object%20Object%20Reference))
  (bind _aspawn (Utilities|Casting|CastToPawn Object))
  (Utilities|FlowControl|Sequence
    (:then_0
      (bind _asbp_beat_em_up_player_state (Utilities|Casting|CastToBP_BeatEmUpPlayerState (Variables|/Script/Engine.Pawn|GetPlayerState _aspawn)))
      (bind _output_get (Variables|/Game/Blueprints/GameplayFramework/BP_BeatEmUpPlayerState.BP_BeatEmUpPlayerState_C|SetCurrentRoom _asbp_beat_em_up_player_state self))
      (bind _outactors (Actor|GetAllActorsOfClass "/Game/Blueprints/Gameplay/BP_PostProcessSkybox.BP_PostProcessSkybox_C"))
      (if (Utilities|Array|IsValidIndex _outactors)
        (Variables|/Game/Blueprints/Gameplay/BP_PostProcessSkybox.BP_PostProcessSkybox_C|SetSkyboxFadeTarget (Utilities|Array|Get(acopy) _outactors) (Math|Float|SelectFloat 1.0 0.0 (Variables|BP_RoomVolume_C|GetShowSky _output_get)))))
    (:then_1
      (Networking|SwitchHasAuthority
        (:Remote
          (if (Pawn|IsLocallyControlled _aspawn)
            (CallFunction|SetLevelState true)
            (for _array_element (Variables|Default|GetConnectedRooms)
              (CallFunction|SetLevelState _array_element true)
              (for _array_element_2 (Variables|Default|GetConnectedRooms)
                (for _array_element_3 (Variables|BP_RoomVolume_C|GetConnectedRooms _array_element_2)
                  (if (and (!= _array_element_3 self) (not (CallFunction|ContainsLocalPawn _array_element_3)))
                    (CallFunction|SetLevelState _array_element_3 false)))))))))))

(fn ActorArrayContainsLocalPawn
  (params (Actors :type Array%20of%20Actor%20Object%20References))
  (for _array_element Actors
    (bind _aspawn (Utilities|Casting|CastToPawn _array_element))
    (if (Pawn|IsLocallyControlled _aspawn)
      (return true)))
  (return false))

(fn ContainsActor
  (params (Actor :type Actor%20Object%20Reference))
  (return (Utilities|Array|ContainsItem (Collision|GetOverlappingActors 0 :!class /Script/Engine.Actor) Actor)))

(fn ConnectedRoomsContainActor
  (params (Actor :type Actor%20Object%20Reference))
  (for _array_element (Variables|Default|GetConnectedRooms)
    (if (Utilities|Array|ContainsItem (Collision|GetOverlappingActors _array_element 0 :!class /Script/Engine.Actor) Actor)
      (return true)))
  (return false))

(fn ContainsLocalPawn
  (for _array_element (Collision|GetOverlappingActors 0 :!class /Script/Engine.Actor)
    (bind _aspawn (Utilities|Casting|CastToPawn _array_element))
    (if (Pawn|IsLocallyControlled _aspawn)
      (return true)))
  (return false))

(fn ConnectedRoomsContainLocalPawn
  (for _array_element (Variables|Default|GetConnectedRooms)
    (if (CallFunction|ContainsLocalPawn _array_element)
      (return true)))
  (return false))