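; Beat-em-up pawn Blueprint that links a Moveset component to character movement and damage reactions.
; Taking damage calls the parent handler and raises a moveset input flag, which the moveset's Damage Reset event clears.
; Moveset events also drive motion: Jump applies a vertical velocity-change impulse, while Set Velocity overwrites movement velocity, flipping Y by sprite direction and rotating it into actor space.
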(event OnMovesetEvent(Moveset)
  (params (EventName :type Name) (EventLocation :type Vector :default "0, 0, 0") (EventDirection :type Vector))
  (bind (_x _y _z) (Math|Vector|BreakVector EventDirection))
  ;[1 1 1] BasicMoveset event handler
  (switch name EventName
    (:Jump
      (CallFunction|ApplyImpulsetoCharacter self (Math|Vector|MakeVector 0.0 0.0 (.Z (Math|Vector|BreakVector EventDirection))) true false))
    (:SetVelocity
      (Variables|/Script/Engine.MovementComponent|SetVelocity (Variables|Default|GetBeatEmUpMovement) (Math|Vector|RotateVector (Math|Vector|MakeVector _x (* _y (CallFunction|GetSpriteDirectionScalar)) _z) (Transformation|GetActorRotation))))
    (:DamageReset
      (CallFunction|SetMovesetInput (Utilities|Enum|LiteralenumBeatEmUpInputSchema "NewEnumerator14") false))))

(event EventTakeDamage
  (params (BaseDamage :type Float%20%28single-precision%29))
  (|CallParentFunction BaseDamage)
  (CallFunction|SetMovesetInput (Utilities|Enum|LiteralenumBeatEmUpInputSchema "NewEnumerator14") true))

(fn ConstructionScript
  (|CallParentFunction))