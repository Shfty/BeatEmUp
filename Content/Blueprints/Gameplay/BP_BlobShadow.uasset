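; Blob shadow actor that projects a decal onto the static world surface beneath it.
; Each Tick it line-traces straight down against WorldStatic objects, moving the decal to the hit point and orienting it along the surface normal.
; When nothing is hit, the decal returns to its default relative position and rotation.
; The construction script uniformly scales the decal by the Radius variable.
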(event EventTick
  (params (DeltaSeconds :type Float%20%28single-precision%29))
  (bind _returnvalue (Transformation|GetActorLocation))
  (bind _decal (Variables|Default|GetDecal))
  (bind (_outhit _returnvalue_2) (Collision|LineTraceForObjects _returnvalue (- _returnvalue "0, 0,10000.000000") (Utilities|Array|MakeArray "ObjectTypeQuery1") false 0 "None"))
  (if _returnvalue_2
    (Transformation|SetWorldLocation _decal (.Location (Collision|BreakHitResult _outhit)) false false)
    (Transformation|SetWorldRotation _decal (Math|Rotator|MakeRotfromX (.Normal (Collision|BreakHitResult _outhit))) false false)
    (else
      (Transformation|SetRelativeLocation _decal "0, 0, 0" false false)
      (Transformation|SetRelativeRotation _decal "0, 0, 0" false false))))

(fn ConstructionScript
  (bind _radius (Variables|Default|GetRadius))
  (Transformation|SetRelativeScale3D (Variables|Default|GetDecal) (Math|Vector|MakeVector _radius _radius _radius)))