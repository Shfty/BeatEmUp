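; Actor component that billboards its owner by matching the owner's yaw to player camera 0's yaw every tick, leaving pitch and roll intact.
; If the root is a primitive component, it rotates horizontal physics velocity by the yaw change since the previous tick, preserving vertical speed, so motion turns with the camera.
; A DoOnce seeds the previous yaw on the first tick to avoid an initial jump.
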(event EventTick
  (params (DeltaSeconds :type Float%20%28single-precision%29))
  (bind _returnvalue (Components|GetOwner))
  (bind _returnvalue_2 (Transformation|GetActorRotation _returnvalue))
  (Utilities|FlowControl|Sequence
    (:then_0
      (bind _output_get (Variables|Default|SetYaw (.yaw (Camera|GetCameraRotation (Game|GetPlayerCameraManager 0)))))
      (Transformation|SetActorRotation _returnvalue (Math|Rotator|MakeRotator (.roll _returnvalue_2) (.pitch _returnvalue_2) _output_get)))
    (:then_1
      (Utilities|FlowControl|DoOnce false
        (:Completed
          (Variables|Default|SetPrevYaw (Variables|Default|GetYaw)))))
    (:then_2
      (bind _asprimitive_component (Utilities|Casting|CastToPrimitiveComponent (VehicleSound|GetRootComponent (Components|GetOwner))))
      (if (!= (- (Variables|Default|GetYaw) (Variables|Default|GetPrevYaw)) 0.0)
        (bind _returnvalue_3 (Physics|GetPhysicsLinearVelocity _asprimitive_component "None"))
        (Physics|SetPhysicsLinearVelocity _asprimitive_component (Math|Vector|MakeVector (.X (Math|Vector|BreakVector (Math|Vector|RotateVectorAroundAxis (Math|Vector|MakeVector (.X (Math|Vector|BreakVector _returnvalue_3)) (.Y (Math|Vector|BreakVector _returnvalue_3)) 0.0) (- (Variables|Default|GetYaw) (Variables|Default|GetPrevYaw)) "0, 0,1.000000"))) (.Y (Math|Vector|BreakVector (Math|Vector|RotateVectorAroundAxis (Math|Vector|MakeVector (.X (Math|Vector|BreakVector _returnvalue_3)) (.Y (Math|Vector|BreakVector _returnvalue_3)) 0.0) (- (Variables|Default|GetYaw) (Variables|Default|GetPrevYaw)) "0, 0,1.000000"))) (.Z (Math|Vector|BreakVector _returnvalue_3))) false "None")))
    (:then_3
      (Variables|Default|SetPrevYaw (Variables|Default|GetYaw)))))