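; Player camera manager for the beat-em-up that follows a target transform supplied by the controlled BP_BeatEmUpPawn.
; Tick interpolates toward that transform on the local player, and the camera update places the view along its right vector, looking back.
; The transform's Y/Z scale doubles as shear factor and offset input.
; Location snaps to whole units when rounded yaw is a 45-degree multiple; other view targets use parent behavior.
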(event EventTick
  (params (DeltaSeconds :type Float%20%28single-precision%29))
  (bind _returnvalue (Game|Player|GetOwningPlayerController))
  (if (Pawn|IsLocalPlayerController _returnvalue)
    (bind _asbp_beat_em_up_pawn (Utilities|Casting|CastToBP_BeatEmUpPawn (Pawn|GetControlledPawn _returnvalue)))
    (Variables|State|Interpolation|SetCameraTransform (Class|KismetMathLibrary|TInterpto (Variables|State|Interpolation|GetCameraTransform) (Variables|/Game/Blueprints/GameplayFramework/BP_BeatEmUpPawn.BP_BeatEmUpPawn_C|GetTargetCameraTransform _asbp_beat_em_up_pawn) (Utilities|Time|GetWorldDeltaSeconds) (Variables|Stats|GetCameraInterpSpeed)))))

(fn ConstructionScript)

(fn BlueprintUpdateCamera
  (params (CameraTarget :type Actor%20Object%20Reference))
  (bind _cameratransform (Variables|State|Interpolation|GetCameraTransform))
  (bind _cameradistance (Variables|Stats|GetCameraDistance))
  (bind (_location _rotation _scale) (Math|Transform|BreakTransform _cameratransform))
  (bind _returnvalue (Math|Vector|GetRightVector _rotation))
  (bind (_x _y _z) (Math|Vector|BreakVector _scale))
  (bind _returnvalue_2 (* _returnvalue _cameradistance))
  (bind _returnvalue_3 (Math|Vector2D|MakeVector2D _y _z))
  (bind _returnvalue_4 (+ _location _returnvalue_2))
  (Utilities|Casting|CastToBP_BeatEmUpPawn CameraTarget
    (:then
      (Class|OrthoHMDFunctionLibrary|SetShearFactor _returnvalue_3)
      (Class|OrthoHMDFunctionLibrary|SetShearOffset (* _returnvalue_3 (* (Variables|Stats|GetShearOffset) -1.0)))
      (return (select (== (Math|Integer|%(Integer) (Math|Float|Round (.Yaw (Math|Rotator|BreakRotator _rotation))) 45) 0) (CallFunction|RoundVector _returnvalue_4) _returnvalue_4) (Math|Rotator|MakeRotfromXZ (* _returnvalue -1.0) (Math|Vector|MakeVector 0.0 0.0 1.0)) 9e+01 true))
    (:CastFailed
      (bind (_newcameralocation _newcamerarotation _newcamerafov _returnvalue_5) (|CallParentFunction CameraTarget))
      (return _newcameralocation _newcamerarotation _newcamerafov _returnvalue_5))))

(fn RoundVector
  (params (InVec :type Vector))
  (bind (_x _y _z) (Math|Vector|BreakVector InVec))
  (return (Math|Vector|MakeVector (Math|Conversions|ToFloat(Integer) (Math|Float|Round _x)) (Math|Conversions|ToFloat(Integer) (Math|Float|Round _y)) (Math|Conversions|ToFloat(Integer) (Math|Float|Round _z)))))