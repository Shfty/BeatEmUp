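; Post-process actor that renders a skybox effect through a blendable material with an adjustable fade.
; The construction script applies the Enabled setting, snaps the fade to its target and adds the base material as a blendable.
; BeginPlay adds a dynamic material instance and forces the post-process on.
; Tick eases SkyboxFade toward its target with FInterpTo, pushing it to the material through UpdateMID while the values differ.
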(event EventBeginPlay
  (bind _returnvalue (Rendering|Material|CreateDynamicMaterialInstance (Variables|Default|GetSkyboxMaterial) :!class /Script/Engine.KismetMaterialLibrary))
  (bind _output_get (Variables|Default|SetSkyboxMID _returnvalue))
  (Rendering|AddorUpdateBlendable (Variables|Default|GetPostProcess) _output_get 1.0 :!class /Script/Engine.PostProcessComponent)
  (CallFunction|UpdateMID)
  (Variables|/Script/Engine.PostProcessComponent|SetbEnabled (Variables|Default|GetPostProcess) true))

(event EventTick
  (params (DeltaSeconds :type Float%20%28single-precision%29))
  (bind _skyboxfadetarget (Variables|Default|GetSkyboxFadeTarget))
  (if (!= (Variables|Default|GetSkyboxFade) _skyboxfadetarget)
    (Variables|Default|SetSkyboxFade (Math|Interpolation|FInterpTo (Variables|Default|GetSkyboxFade) _skyboxfadetarget DeltaSeconds (Variables|Default|GetSkyboxFadeSpeed)))
    (CallFunction|UpdateMID)))

(fn ConstructionScript
  (Variables|/Script/Engine.PostProcessComponent|SetbEnabled (Variables|Default|GetPostProcess) (Variables|Default|GetEnabled))
  (Variables|Default|SetSkyboxFade (Variables|Default|GetSkyboxFadeTarget))
  (Rendering|AddorUpdateBlendable (Variables|Default|GetPostProcess) (Variables|Default|GetSkyboxMaterial) 1.0 :!class /Script/Engine.PostProcessComponent))

(fn UpdateMID
  (Rendering|Material|SetScalarParameterValue (Variables|Default|GetSkyboxMID) "SkyboxFade" (Variables|Default|GetSkyboxFade) :!class /Script/Engine.MaterialInstanceDynamic))