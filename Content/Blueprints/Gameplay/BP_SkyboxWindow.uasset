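; BP_SkyboxWindow is a resizable window actor with an optional point light, whose mesh is excluded from the main render pass at BeginPlay.
; The construction script scales the mesh to WindowExtent and calls ConfigurePointLight.
; When the light is enabled, its source length, radius and Z offset derive from the window extent, with exposed intensity and attenuation; otherwise all its settings receive default inputs.
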(event EventBeginPlay
  (Class|PrimitiveComponent|SetRenderinMainPass (Variables|Default|GetStaticMesh) false))

(fn ConstructionScript
  (bind _windowextent (Variables|Default|GetWindowExtent))
  (bind _windowextent_2 (Variables|Default|GetWindowExtent))
  (bind _returnvalue (* (.y _windowextent) 0.5))
  (Utilities|FlowControl|Sequence
    (:then_0
      (Transformation|SetWorldScale3D (Variables|Default|GetStaticMesh) (Math|Vector|MakeVector (.x _windowextent_2) (.y _windowextent_2) 1.0)))
    (:then_1
      (if (Variables|Default|GetPointLightEnabled)
        (CallFunction|ConfigurePointLight (Variables|Default|GetLightIntensity) (Variables|Default|GetLightAttenuationRadius) (- (.x _windowextent) _returnvalue) (.y _windowextent) _returnvalue)
        (else
          (CallFunction|ConfigurePointLight 0.0 0.0 0.0 0.0 0.0))))))

(fn ConfigurePointLight
  (params (Intensity :type Float%20%28single-precision%29) (AttenuationRadius :type Float%20%28single-precision%29) (SourceLength :type Float%20%28single-precision%29) (SourceRadius :type Float%20%28single-precision%29) (ZOffset :type Float%20%28single-precision%29))
  (bind _pointlight (Variables|Default|GetPointLight))
  (Class|PointLightComponent|SetSourceRadius _pointlight SourceRadius)
  (Class|PointLightComponent|SetSourceLength _pointlight SourceLength)
  (Rendering|Components|Light|SetIntensity _pointlight Intensity)
  (Rendering|Lighting|SetAttenuationRadius _pointlight AttenuationRadius)
  (Transformation|SetRelativeLocation _pointlight (Math|Vector|MakeVector 0.0 0.0 ZOffset) false false))