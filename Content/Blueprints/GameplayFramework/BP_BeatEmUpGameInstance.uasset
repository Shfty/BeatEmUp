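; Game instance for the beat 'em up that keeps audio volume settings in a save game and applies them at startup.
; On Init it loads the saved settings, then after a short delay overrides master, effects and music sound class volumes in the sound mix, or saves defaults if loading fails.
; Load and save helpers lazily create the save object to get its slot.
; Network and travel errors are printed on screen.
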(event Custom|UpdateAudioSettings
  (bind _audiosettingssavegame (Variables|Default|GetAudioSettingsSaveGame))
  (Audio|SetSoundMixClassOverride "/Game/Audio/SM_BeatEmUpSoundMix.SM_BeatEmUpSoundMix" "/Game/Audio/SC_Master.SC_Master" (Variables|/Game/Blueprints/GameplayFramework/BP_AudioSettingsSaveGame.BP_AudioSettingsSaveGame_C|GetMasterVolume _audiosettingssavegame) 1.0 0.0 true)
  (Audio|SetSoundMixClassOverride "/Game/Audio/SM_BeatEmUpSoundMix.SM_BeatEmUpSoundMix" "/Game/Audio/SC_Effects.SC_Effects" (Variables|/Game/Blueprints/GameplayFramework/BP_AudioSettingsSaveGame.BP_AudioSettingsSaveGame_C|GetEffectsVolume _audiosettingssavegame) 1.0 0.0 false)
  (Audio|SetSoundMixClassOverride "/Game/Audio/SM_BeatEmUpSoundMix.SM_BeatEmUpSoundMix" "/Game/Audio/SC_Music.SC_Music" (Variables|/Game/Blueprints/GameplayFramework/BP_AudioSettingsSaveGame.BP_AudioSettingsSaveGame_C|GetMusicVolume _audiosettingssavegame) 1.0 0.0 false))

(event EventHandleNetworkError
  (params (FailureType :type ENetworkFailure%20Enum :default "NetDriverAlreadyExists") (bIsServer :type Boolean))
  (Development|PrintString (Utilities|String|Append "Network Error: " (Utilities|String|EnumtoString FailureType) " (" (Utilities|String|SelectString "Client" "Server" bIsServer) ")")))

(event EventHandleTravelError
  (params (FailureType :type ETravelFailure%20Enum :default "NoLevel"))
  (Development|PrintString (Utilities|String|Append "Travel Error: " (Utilities|String|EnumtoString FailureType))))

(event EventInit
  (bind _success (CallFunction|LoadAudioSettings))
  (if _success
    (Utilities|FlowControl|Delay 0.2)
    (CallFunction|UpdateAudioSettings)
    (else
      (CallFunction|SaveAudioSettings))))

(fn GetAudioSettingsSaveGame
  (Utilities|IsValid (Variables|Default|GetAudioSettingsSaveGame)
    (:Is%20Valid
      (return (Variables|Default|GetAudioSettingsSaveGame)))
    (:Is%20Not%20Valid
      (bind _returnvalue (SaveGame|CreateSaveGameObject "/Game/Blueprints/GameplayFramework/BP_AudioSettingsSaveGame.BP_AudioSettingsSaveGame_C"))
      (bind _output_get (Variables|Default|SetAudioSettingsSaveGame _returnvalue))
      (return _output_get))))

(fn LoadAudioSettings
  (bind _audiosettingssavegame (CallFunction|GetAudioSettingsSaveGame))
  (bind _returnvalue (SaveGame|LoadGamefromSlot (Variables|/Game/Blueprints/GameplayFramework/BP_AudioSettingsSaveGame.BP_AudioSettingsSaveGame_C|GetSaveSlotName _audiosettingssavegame) (Variables|/Game/Blueprints/GameplayFramework/BP_AudioSettingsSaveGame.BP_AudioSettingsSaveGame_C|GetSaveSlotIndex _audiosettingssavegame)))
  (bind _asbp_audio_settings_save_game (Utilities|Casting|CastToBP_AudioSettingsSaveGame _returnvalue)
    (:then
      (bind _output_get (Variables|Default|SetAudioSettingsSaveGame _asbp_audio_settings_save_game))
      (return _output_get true))
    (:CastFailed
      (return 0 false))))

(fn SaveAudioSettings
  (bind _audiosettingssavegame (CallFunction|GetAudioSettingsSaveGame))
  (bind _returnvalue (SaveGame|SaveGametoSlot _audiosettingssavegame (Variables|/Game/Blueprints/GameplayFramework/BP_AudioSettingsSaveGame.BP_AudioSettingsSaveGame_C|GetSaveSlotName _audiosettingssavegame) (Variables|/Game/Blueprints/GameplayFramework/BP_AudioSettingsSaveGame.BP_AudioSettingsSaveGame_C|GetSaveSlotIndex _audiosettingssavegame)))
  (return _returnvalue))