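; Beat 'em up GameState that drives a fixed-timestep simulation clock independent of render frame rate.
; BeginPlay sets the frame rate limit to zero, and Tick accumulates delta time.
; A looped-back Sequence calls CallFixedTick and increments CurrentFrame for each whole timestep accumulated, carrying the remainder over.
; A ServerFrame RepNotify exists but is empty.
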(event EventBeginPlay
  (CallFunction|SetFramerateLimit))

(event EventTick
  (params (DeltaSeconds :type Float%20%28single-precision%29))
  ;[1 1 1] Fixed timestep tick
  (bind _output_get (Variables|FixedTick|SetFixedTimestepAccumulator (+ (Variables|FixedTick|GetFixedTimestepAccumulator) DeltaSeconds)))
  (if (>= _output_get (Variables|FixedTick|GetFixedTimestep)) :!label _label
    (Utilities|FlowControl|Sequence
      (:then_0
        (Default|CallFixedTick)
        (Math|Integer|IncrementInt (Variables|Default|GetCurrentFrame)))
      (:then_1
        (Variables|FixedTick|SetFixedTimestepAccumulator (- (Variables|FixedTick|GetFixedTimestepAccumulator) (Variables|FixedTick|GetFixedTimestep))))
      (:then_2
        (goto _label)))))

(fn ConstructionScript)

(fn OnRepServerFrame)